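; Camera component that toggles a free-look camera on its owner's spring arm, which it gets through a GetSpringArmMessage call.
; Entering free cam turns off spring arm rotation inheritance, and Tick applies the accumulated yaw and clamped pitch, scaled by sensitivity, as relative rotation.
; Toggling off restores inheritance and flags a reset, which blocks look input until the next Tick snaps rotation to zero and clears the state.
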(event EventSetSpringArmInherit
  (params (Value :type Boolean))
  (bind _value (Class|BPIShipData|GetSpringArm(Message) (Components|GetOwner)))
  (Variables|/Script/Engine.SpringArmComponent|SetbInheritPitch _value Value)
  (Variables|/Script/Engine.SpringArmComponent|SetbInheritRoll _value Value)
  (Variables|/Script/Engine.SpringArmComponent|SetbInheritYaw _value Value))

(event EventSetCameraPitch
  (params (Value :type Float%20%28double-precision%29))
  (if (not (Variables|Default|GetResettingCam))
    (Variables|Default|SetCameraPitch (Math|Float|Clamp(Float) (+ (Variables|Default|GetCameraPitch) (* Value (Variables|Default|GetCameraSens))) -8e+01 8e+01))))

(event EventSetCameraYaw
  (params (Value :type Float%20%28double-precision%29))
  (if (not (Variables|Default|GetResettingCam))
    (Variables|Default|SetCameraYaw (+ (Variables|Default|GetCameraYaw) (* Value (Variables|Default|GetCameraSens))))))

(event EventTick
  (params (DeltaSeconds :type Float%20%28single-precision%29))
  (CallFunction|HandleResetCamera)
  (Utilities|IsFreeCam
    (:true
      (CallFunction|HandleFreeCamera))))

(event EventToggleFreeCam
  (Utilities|IsFreeCam
    (:true
      (Variables|Default|SetResettingCam true)
      (CallFunction|SetSpringArmInherit true))
    (:false
      (Variables|Default|SetFreeCam true)
      (CallFunction|SetSpringArmInherit false))))

(fn HandleFreeCamera
  (bind _value (Class|BPIShipData|GetSpringArm(Message) (Components|GetOwner)))
  (Transformation|SetRelativeRotation _value (Math|Rotator|MakeRotator 0.0 (Variables|Default|GetCameraPitch) (Variables|Default|GetCameraYaw)) false false))

(fn HandleResetCamera
  (Utilities|IsResettingCam
    (:true
      (bind _value (Class|BPIShipData|GetSpringArm(Message) (Components|GetOwner)))
      (Transformation|SetRelativeRotation _value "0, 0, 0" false false)
      (Variables|Default|SetResettingCam false)
      (Variables|Default|SetCameraYaw 0.0)
      (Variables|Default|SetCameraPitch 0.0)
      (Variables|Default|SetFreeCam false))))

(fn GetIsFreeCam
  (return (Variables|Default|GetFreeCam)))