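; Ship component that auto-levels its owner while the stabilizer is enabled.
; Each tick it picks an up normal: world up in space, otherwise the impact normal of a downward line trace, switching itself off if nothing is hit.
; It eases rotation toward that normal with RInterpTo and MakeRotFromZX, using the ship body's forward vector for heading.
; Toggling works only while the ship is online; otherwise it forces the stabilizer off.
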(event EventSetComponent
  (params (Value :type Boolean))
  (Variables|Default|SetStabilizerEnabled Value))

(event EventToggleComponent
  (Utilities|IsShipOnline
    (:true
      (Variables|Default|SetStabilizerEnabled (not (Variables|Default|GetStabilizerEnabled))))
    (:false
      (Variables|Default|SetStabilizerEnabled false))))

(event EventTickComponent
  (params (DeltaTime :type Float%20%28double-precision%29))
  (bind _returnvalue (Components|GetOwner))
  (Utilities|IsStabilizerEnabled
    (:true
      (CallFunction|SetStabilizerNormal)
      (bind _value (Class|BPIShipData|GetShipStatus(Message) _returnvalue))
      (Transformation|SetActorRotation _returnvalue (Math|Interpolation|RInterpTo (Transformation|GetActorRotation _returnvalue) (Math|Rotator|MakeRotfromZX (Variables|Default|GetStabilizerNormal) (Math|Vector|GetForwardVector (Utilities|Struct|BreakS_ShipData _value))) (Utilities|Time|GetWorldDeltaSeconds) (Utilities|Struct|BreakS_StabilizerConfig (Variables|Default|GetStabilizerConfig)))))))

(fn SetStabilizerNormal
  (bind _returnvalue (Components|GetOwner))
  (bind _returnvalue_2 (Transformation|GetActorLocation _returnvalue))
  (Utilities|IsShipinSpace
    (:true
      (Variables|Default|SetStabilizerNormal "0.000000,0.000000,1.000000"))
    (:false
      (bind (_outhit _returnvalue_3) (Collision|LineTraceByChannel _returnvalue_2 (+ _returnvalue_2 (* (Math|Vector|VectorUp) -1.0 (Utilities|Struct|BreakS_StabilizerConfig (Variables|Default|GetStabilizerConfig)))) "TraceTypeQuery1" false 0 "None" true "(R=1.000000,G=0.000000,B=0.000000,A=1.000000)" "(R=0.000000,G=1.000000,B=0.000000,A=1.000000)" 4.0))
      (if _returnvalue_3
        (Variables|Default|SetStabilizerNormal (.ImpactNormal (Collision|BreakHitResult _outhit)))
        (else
          (Variables|Default|SetStabilizerEnabled false))))))