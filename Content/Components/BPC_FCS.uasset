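; BPC_FCS is a component, likely a flight control system, that balances thruster output between opposing sides.
; BalanceThrusters totals thrust per side from the thruster data array, then derives horizontal and vertical limit factors from weak-to-strong ratios, blended by FCSStrength.
; It scales down each thruster on the stronger side of left/right and top/bottom pairs.
; The FCSEnabled macro gates this, returning the data unchanged when disabled.
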(fn BalanceThrusters
  (params (RawData :type Array%20of%20S%20Thruster%20Data%20Structures))
  (Utilities|FCSEnabled
    (:true
      (for _array_element RawData
        (switch Utilities|FlowControl|Switch|SwitchonE_ThrusterSide (.Side (Utilities|Struct|BreakS_ThrusterData _array_element))
          (:NewEnumerator0
            (LocalVariables|SetTotalThrustLeft (+ (LocalVariables|GetTotalThrustLeft) (.Thrust (Utilities|Struct|BreakS_ThrusterData _array_element)))))
          (:NewEnumerator1
            (LocalVariables|SetTotalThrustRight (+ (LocalVariables|GetTotalThrustRight) (.Thrust (Utilities|Struct|BreakS_ThrusterData _array_element)))))
          (:NewEnumerator2
            (LocalVariables|SetTotalThrustTop (+ (LocalVariables|GetTotalThrustTop) (.Thrust (Utilities|Struct|BreakS_ThrusterData _array_element)))))
          (:NewEnumerator3
            (LocalVariables|SetTotalThrustBottom (+ (LocalVariables|GetTotalThrustBottom) (.Thrust (Utilities|Struct|BreakS_ThrusterData _array_element)))))))
      (Utilities|FlowControl|Sequence
        (:then_0
          (LocalVariables|SetWeakSideHorizontal (Math|Float|Min(Float) (LocalVariables|GetTotalThrustLeft) (LocalVariables|GetTotalThrustRight)))
          (LocalVariables|SetStrongSideHorizontal (Math|Float|Max(Float) (LocalVariables|GetTotalThrustLeft) (LocalVariables|GetTotalThrustRight)))
          (LocalVariables|SetLimitFactorHorizontal (Math|Float|Lerp 1.0 (/ (LocalVariables|GetWeakSideHorizontal) (LocalVariables|GetStrongSideHorizontal)) (Variables|Default|GetFCSStrength))))
        (:then_1
          (LocalVariables|SetWeakSideVertical (Math|Float|Min(Float) (LocalVariables|GetTotalThrustTop) (LocalVariables|GetTotalThrustBottom)))
          (LocalVariables|SetStrongSideVertical (Math|Float|Max(Float) (LocalVariables|GetTotalThrustTop) (LocalVariables|GetTotalThrustBottom)))
          (LocalVariables|SetLimitFactorVertical (Math|Float|Lerp 1.0 (/ (LocalVariables|GetWeakSideVertical) (LocalVariables|GetStrongSideVertical)) (Variables|Default|GetFCSStrength))))
        (:then_2
          (for (_array_element_2 _array_index) RawData
            (Utilities|FlowControl|Sequence
              (:then_0
                (if (and (Utilities|Enum|Equal(Enum) (.Side (Utilities|Struct|BreakS_ThrusterData _array_element_2)) "NewEnumerator0") (> (LocalVariables|GetTotalThrustLeft) (LocalVariables|GetTotalThrustRight)))
                  (bind _structout (Utilities|Struct|SetmembersinS_ThrusterData _array_element_2 (* (.Thrust (Utilities|Struct|BreakS_ThrusterData _array_element_2)) (LocalVariables|GetLimitFactorHorizontal)) :!label _label))
                  (Utilities|Array|SetArrayElem RawData _array_index _structout)))
              (:then_1
                (if (and (Utilities|Enum|Equal(Enum) (.Side (Utilities|Struct|BreakS_ThrusterData _array_element_2)) "NewEnumerator1") (> (LocalVariables|GetTotalThrustRight) (LocalVariables|GetTotalThrustLeft)))
                  (goto _label)))
              (:then_2
                (if (and (Utilities|Enum|Equal(Enum) (.Side (Utilities|Struct|BreakS_ThrusterData _array_element_2)) "NewEnumerator2") (> (LocalVariables|GetTotalThrustTop) (LocalVariables|GetTotalThrustBottom)))
                  (bind _structout_2 (Utilities|Struct|SetmembersinS_ThrusterData _array_element_2 (* (.Thrust (Utilities|Struct|BreakS_ThrusterData _array_element_2)) (LocalVariables|GetLimitFactorVertical)) :!label _label_2))
                  (Utilities|Array|SetArrayElem RawData _array_index _structout_2)))
              (:then_3
                (if (and (Utilities|Enum|Equal(Enum) (.Side (Utilities|Struct|BreakS_ThrusterData _array_element_2)) "NewEnumerator3") (> (LocalVariables|GetTotalThrustBottom) (LocalVariables|GetTotalThrustTop)))
                  (goto _label_2)))))
          (return RawData))))
    (:false
      (return RawData))))