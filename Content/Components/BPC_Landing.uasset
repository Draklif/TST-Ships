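; Actor component that handles landing and launching for its owning ship, talking to it through message calls.
; InitSequence branches on the ship's landed state to launch or land.
; Launch applies an upward impulse, disables gravity and powers on, while landing powers off and restores gravity only if a debug-drawn downward trace finds a surface within range.
; A toggleable landing-enabled flag has its own check macro, but InitSequence does not consult it.
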(event EventSetLanding
  (params (Value :type Boolean))
  (Variables|Default|SetLandingEnabled Value))

(event EventToggleLanding
  (Variables|Default|SetLandingEnabled (not (Variables|Default|GetLandingEnabled))))

(event EventLandSequence
  (bind _returnvalue (Components|GetOwner))
  (bind _returnvalue_2 (Components|GetOwner))
  (bind _returnvalue_3 (Transformation|GetActorLocation _returnvalue_2))
  (bind _returnvalue_4 (Collision|LineTraceByChannel _returnvalue_3 (+ _returnvalue_3 (Math|Vector|MakeVector 0.0 0.0 (* (Utilities|Struct|BreakS_LandingConfig (Variables|Default|GetLandingConfig)) -1.0))) "TraceTypeQuery1" false 0 "ForDuration" true "(R=1.000000,G=0.000000,B=0.863777,A=1.000000)"))
  (if _returnvalue_4
    (bind _value (Class|BPIShipData|GetShipStatus(Message) _returnvalue))
    (Physics|SetEnableGravity (Utilities|Struct|BreakS_ShipData _value) true)
    (Class|BPIShipControls|PowerOff(Message) _returnvalue)
    (Class|BPIShipControls|SetIsLanded(Message) (Components|GetOwner) true)))

(event EventLaunchSequence
  (bind _returnvalue (Components|GetOwner))
  (bind _value (Class|BPIShipData|GetShipStatus(Message) _returnvalue))
  (Physics|AddImpulse (Utilities|Struct|BreakS_ShipData _value) (Math|Vector|MakeVector 0.0 0.0 (* (Utilities|Struct|BreakS_LandingConfig (Variables|Default|GetLandingConfig)) (Utilities|Time|GetWorldDeltaSeconds))) "None" true)
  (Physics|SetEnableGravity (Utilities|Struct|BreakS_ShipData _value) false)
  (Class|BPIShipControls|Poweron(Message) _returnvalue)
  (Class|BPIShipControls|SetIsLanded(Message) (Components|GetOwner) false))

(event EventInitSequence
  (Utilities|IsShipLanded
    (:true
      (CallFunction|LaunchSequence))
    (:false
      (CallFunction|LandSequence))))