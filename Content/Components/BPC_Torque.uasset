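; Ship component that turns pitch, yaw and roll input into physics torque on the owning ship's body.
; Each tick, a ship flag selects full control strength or the configured reduced "off" strength.
; Rotation input is applied only while torque is enabled and the ship is outside a specific location state.
; Torque acts around the body's local axes as mass-independent acceleration, scaled by per-axis config and control strength.
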(event EventTick
  (params (DeltaSeconds :type Float%20%28single-precision%29))
  (Utilities|CheckShipFlag "NewEnumerator0"
    (:true
      (Variables|Default|SetControlStrength 1.0))
    (:false
      (Variables|Default|SetControlStrength (Utilities|Struct|BreakS_TorqueConfig (Variables|Config|GetTorqueConfig))))))

(event EventHandleRotation
  (params (Value :type Float%20%28double-precision%29) (Axis :type E_Rotation%20Enum :default "NewEnumerator0"))
  (Utilities|CheckShipLocationState "NewEnumerator0"
    (:false
      (Utilities|IsTorqueEnabled
        (:true
          (CallFunction|AddTorque Value Axis))))))

(event EventSetComponent
  (params (Value :type Boolean))
  (Variables|Flags|SetTorqueEnabled Value))

(event EventToggleComponent
  (Variables|Flags|SetTorqueEnabled (not (Variables|Flags|GetTorqueEnabled))))

(fn AddTorque
  (params (Value :type Float%20%28double-precision%29) (Axis :type E_Rotation%20Enum :default "NewEnumerator0"))
  (bind _torqueconfig (Variables|Config|GetTorqueConfig))
  (bind (_pitchstrength _yawstrength _rollstrength) (Utilities|Struct|BreakS_TorqueConfig _torqueconfig))
  (bind _value (Class|BPIShipData|GetShipStatus(Message) (Components|GetOwner)))
  (Class|PrimitiveComponent|AddTorqueinDegrees (.Body (Utilities|Struct|BreakS_ShipData _value)) (* (* Value (Utilities|Select :Index Axis :NewEnumerator0 _pitchstrength :NewEnumerator2 _yawstrength :NewEnumerator1 _rollstrength) (Variables|Default|GetControlStrength)) (Utilities|Select :Index Axis :NewEnumerator0 (Math|Vector|GetRightVector (.Body (Utilities|Struct|BreakS_ShipData _value))) :NewEnumerator2 (Math|Vector|GetUpVector (.Body (Utilities|Struct|BreakS_ShipData _value))) :NewEnumerator1 (Math|Vector|GetForwardVector (.Body (Utilities|Struct|BreakS_ShipData _value))))) "None" true))