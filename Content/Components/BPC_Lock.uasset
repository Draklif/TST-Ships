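; Ship component that locks onto a planet or moon and turns the owning ship to face it.
; Toggling on picks the BPI_Lockable actor projected nearest screen center, requires the ship online and in space, and switches off the stabilizer.
; LockTick eases rotation toward the target's lock-on point at LockStrength, using the ship's up vector.
; Ship status, target data and stabilizer control go through message calls.
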(event EventSetComponent
  (params (Value :type Boolean))
  (CallFunction|SetLock Value))

(event EventToggleComponent
  (CallFunction|ToggleLock))

(event EventSetLock
  (params (Value :type Boolean))
  (bind _output_get (Variables|Default|SetLockEnabled Value))
  (if (not _output_get)
    (Variables|Default|SetLockTarget 0)))

(event EventToggleLock
  (Utilities|IsShipOnline
    (:true
      (if (Variables|Default|GetLockEnabled)
        (Variables|Default|SetLockTarget 0 :!label _label)
        (Variables|Default|SetLockEnabled false)
        (else
          (bind _lockontarget (CallFunction|FindLockonTarget))
          (bind _output_get (Variables|Default|SetLockTarget _lockontarget))
          (bind _type (Class|BPILockable|GetLockType(Message) _output_get))
          (switch Utilities|FlowControl|Switch|SwitchonE_BodyType _type
            (:NewEnumerator0
              _)
            (:NewEnumerator6
              _))
          (Utilities|IsShipinSpace
            (:true
              (Variables|Default|SetLockEnabled true)
              (Class|BPIShipControls|SetRemoteComponent(Message) (Components|GetOwner) "/Game/Components/BPC_Stabilizer.BPC_Stabilizer_C" false))
            (:false
              (goto _label))))))
    (:false
      (Variables|Default|SetLockEnabled false))))

(event EventLockTick
  (bind _returnvalue (Components|GetOwner))
  (Utilities|IsLockEnabled
    (:true
      (bind _location (Class|BPILockable|GetLockonLocation(Message) (Variables|Default|GetLockTarget)))
      (Transformation|SetActorRotation _returnvalue (Math|Interpolation|RInterpTo (Transformation|GetActorRotation _returnvalue) (Math|Rotator|MakeRotfromZX (Transformation|GetActorUpVector _returnvalue) (Math|Vector|Normalize (- _location (Transformation|GetActorLocation _returnvalue)))) (Utilities|Time|GetWorldDeltaSeconds) (Variables|Default|GetLockStrength))))))

(fn FindLockonTarget
  (LocalVariables|SetScreenCenter (/ (Viewport|GetViewportSize) 2.0))
  (LocalVariables|SetBestTarget 0)
  (LocalVariables|SetBestDistance 999999.0)
  (bind _outactors (Actor|GetAllActorswithInterface "/Game/Components/BPI_Lockable.BPI_Lockable_C"))
  (for _array_element _outactors
    (if (.ReturnValue (Class|GameplayStatics|ProjectWorldtoScreen (Game|GetPlayerController 0) (Transformation|GetActorLocation _array_element) false))
      (if (< (Math|Vector2D|Vector2DLength (- (.ScreenPosition (Class|GameplayStatics|ProjectWorldtoScreen (Game|GetPlayerController 0) (Transformation|GetActorLocation _array_element) false)) (LocalVariables|GetScreenCenter))) (LocalVariables|GetBestDistance))
        (LocalVariables|SetBestDistance (Math|Vector2D|Vector2DLength (- (.ScreenPosition (Class|GameplayStatics|ProjectWorldtoScreen (Game|GetPlayerController 0) (Transformation|GetActorLocation _array_element) false)) (LocalVariables|GetScreenCenter))))
        (LocalVariables|SetBestTarget _array_element))))
  (return (LocalVariables|GetBestTarget)))

(fn IsTargetLocked
  (Utilities|IsLockEnabled
    (:true
      (return true (Variables|Default|GetLockTarget)))
    (:false
      (return false 0))))