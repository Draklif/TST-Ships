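; Ship component that tracks drive and lift thrust power and passes it to the owner's thruster units.
; On BeginPlay it collects child actors implementing BPI_ThrusterUnit from the owner's ChildActorComponents.
; Input raises or lowers clamped power at configured rates while thrust is enabled; zero events ease it back using dampening.
; GetThrusterData sends both powers to each unit and returns their collected data.
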(event EventBeginPlay
  (for _array_element (Actor|GetComponentsByClass (Components|GetOwner) "/Script/Engine.ChildActorComponent")
    (if (Utilities|DoesObjectImplementInterface (Variables|/Script/Engine.ChildActorComponent|GetChildActor _array_element) "/Game/Components/BPI_ThrusterUnit.BPI_ThrusterUnit_C")
      (Utilities|Array|Add (Variables|Default|GetThrusterUnits) (Variables|/Script/Engine.ChildActorComponent|GetChildActor _array_element)))))

(event EventSetComponent
  (params (Value :type Boolean))
  (Variables|Flags|SetIsThrustEnabled Value))

(event EventSetDriveZero
  (Variables|Default|SetDrivePower (Math|Interpolation|FInterpTo (Variables|Default|GetDrivePower) 0.0 (Utilities|Time|GetWorldDeltaSeconds) (Utilities|Struct|BreakS_ShipThrustConfig (Variables|Config|GetShipThrustConfig)))))

(event EventSetLiftZero
  (Variables|Default|SetLiftPower (Math|Interpolation|FInterpTo (Variables|Default|GetLiftPower) 0.0 (Utilities|Time|GetWorldDeltaSeconds) (Utilities|Struct|BreakS_ShipThrustConfig (Variables|Config|GetShipThrustConfig)))))

(event EventSetLiftPower
  (params (LiftInput :type Float%20%28double-precision%29))
  (Utilities|ThrustEnabled
    (:true
      (Variables|Default|SetLiftPower (Math|Float|Clamp(Float) (+ (Variables|Default|GetLiftPower) (* LiftInput (Utilities|Struct|BreakS_ShipThrustConfig (Variables|Config|GetShipThrustConfig)) (Utilities|Time|GetWorldDeltaSeconds))) -1.0)))))

(event EventSetDrivePower
  (params (DriveInput :type Float%20%28double-precision%29))
  (Utilities|ThrustEnabled
    (:true
      (Variables|Default|SetDrivePower (Math|Float|Clamp(Float) (+ (Variables|Default|GetDrivePower) (* DriveInput (Utilities|Struct|BreakS_ShipThrustConfig (Variables|Config|GetShipThrustConfig)) (Utilities|Time|GetWorldDeltaSeconds))))))))

(event EventToggleComponent
  (Variables|Flags|SetIsThrustEnabled (not (Variables|Flags|GetIsThrustEnabled))))

(fn GetThrusterData
  (for _array_element (Variables|Default|GetThrusterUnits)
    (bind _thrusterdata (Class|BPIThrusterUnit|GetThrusterData(Message) _array_element (Variables|Default|GetDrivePower) (Variables|Default|GetLiftPower)))
    (Utilities|Array|Add (LocalVariables|GetThrusterData) _thrusterdata))
  (return (LocalVariables|GetThrusterData)))