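; Ship component that warps the owning ship toward its locked target.
; ToggleWarp requires an online ship and a BPC_Lock target, then starts or cancels a launch timer, setting lock and warp flags through owner messages.
; WarpStart impulses the body toward the target, fades the camera to white, then teleports the owner to a point computed from target type.
; WarpEnd fades back and clears the flags; Tick prints the launch timer.
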(event Custom|Warp%20Start
  (bind _returnvalue (Components|GetOwner))
  (Utilities|Time|ClearandInvalidateTimerbyHandle (Variables|Default|GetWarpLaunchTimer))
  (bind _value (Class|BPIShipData|GetShipStatus(Message) _returnvalue))
  (Physics|AddImpulse (.Body (Utilities|Struct|BreakS_ShipData _value)) (* (CallFunction|FindDirectiontoTarget (.Body (Utilities|Struct|BreakS_ShipData _value))) 3e+04) "None" true)
  (CameraFades|StartCameraFade (Game|GetPlayerCameraManager 0) 0.0 1.0 0.3 "(R=1.000000,G=1.000000,B=1.000000,A=1.000000)" true true)
  (bind _returnvalue_2 (Utilities|Time|SetTimerbyEvent (delegate Custom|Warp%20End) 2.0))
  (Variables|Default|SetWarpTravelTimer _returnvalue_2)
  (Utilities|FlowControl|Delay 1.0)
  (Transformation|SetActorLocation _returnvalue (CallFunction|FindTeleportPoint (.Body (Utilities|Struct|BreakS_ShipData _value))) false false))

(event Custom|Warp%20End
  (bind _returnvalue (Components|GetOwner))
  (Utilities|Time|ClearandInvalidateTimerbyHandle (Variables|Default|GetWarpTravelTimer))
  (CameraFades|StartCameraFade (Game|GetPlayerCameraManager 0) 1.0 0.0 0.3 "(R=1.000000,G=1.000000,B=1.000000,A=1.000000)" true false)
  (Class|BPIShipControls|SetIsLocked(Message) _returnvalue false)
  (Class|BPIShipControls|SetIsWarping(Message) _returnvalue false))

(event EventSetComponent
  (params (Value :type Boolean)))

(event EventToggleComponent)

(event EventToggleWarp
  (bind _returnvalue (Components|GetOwner))
  (bind _returnvalue_2 (Components|GetOwner))
  (Utilities|CanWarp
    (:true
      (Utilities|IsShipWarping
        (:true
          (Utilities|Time|ClearandInvalidateTimerbyHandle (Variables|Default|GetWarpLaunchTimer))
          (Class|BPIShipControls|SetIsLocked(Message) _returnvalue false)
          (Class|BPIShipControls|SetIsWarping(Message) _returnvalue false))
        (:false
          (bind _returnvalue_3 (Utilities|Time|SetTimerbyEvent (delegate Custom|Warp%20Start) 5.0))
          (Variables|Default|SetWarpLaunchTimer _returnvalue_3)
          (Class|BPIShipControls|SetIsLocked(Message) _returnvalue_2 true)
          (Class|BPIShipControls|SetIsWarping(Message) _returnvalue_2 true))))))

(event EventTick
  (params (DeltaSeconds :type Float%20%28single-precision%29))
  (bind _warplaunchtimer (Variables|Default|GetWarpLaunchTimer))
  (if (Utilities|Time|IsValidTimerHandle _warplaunchtimer)
    (Development|PrintString (Utilities|String|ToString(Float) (Class|KismetSystemLibrary|GetTimerElapsedTimeHandle _warplaunchtimer)))))

(fn FindDirectiontoTarget
  (params (Ship :type Scene%20Component%20Object%20Reference))
  (return (Math|Vector|Normalize (- (Transformation|GetActorLocation (Variables|Default|GetLockTarget)) (Transformation|GetWorldLocation Ship)))))

(fn FindTeleportPoint
  (params (Ship :type Scene%20Component%20Object%20Reference))
  (bind _locktarget (Variables|Default|GetLockTarget))
  (bind _type (Class|BPILockable|GetLockType(Message) _locktarget))
  (switch Utilities|FlowControl|Switch|SwitchonE_BodyType _type
    (:NewEnumerator0
      (Variables|Default|SetStopDistance 2e+03)
      (return (- (Transformation|GetActorLocation _locktarget) (* (CallFunction|FindDirectiontoTarget Ship) (Variables|Default|GetStopDistance)))))
    (:NewEnumerator5
      _)
    (:NewEnumerator1
      _)
    (:NewEnumerator6
      _))
  (Variables|Default|SetStopDistance 2e+04))