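; Ship hover component that applies gravity-scaled vertical impulses to the owning ship's body while hover is enabled.
; Each tick it reads the owner's ship status through gate macros and acts only when online, airborne and not in space, using a mass-independent velocity change.
; Toggling requires an online, unlanded ship and switches hover off when offline, while SetHover writes the flag directly.
; Generic SetComponent and ToggleComponent events forward to these.
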(event EventSetComponent
  (params (Value :type Boolean))
  (CallFunction|SetHover Value))

(event EventToggleComponent
  (CallFunction|ToggleHover))

(event EventTick
  (params (DeltaSeconds :type Float%20%28single-precision%29))
  (Utilities|IsHoverEnabled
    (:true
      (Utilities|IsShipOnline
        (:true
          (Utilities|IsShipLanded
            (:false
              (Utilities|IsShipinSpace
                (:false
                  (bind _value (Class|BPIShipData|GetShipStatus(Message) (Components|GetOwner)))
                  (Physics|AddImpulse (.Body (Utilities|Struct|BreakS_ShipData _value)) (Math|Vector|MakeVector 0.0 0.0 (* (.Gravity (Utilities|Struct|BreakS_ShipData _value)) DeltaSeconds)) "None" true))))))))))

(event EventToggleHover
  (Utilities|IsShipOnline
    (:true
      (Utilities|IsShipLanded
        (:false
          (Variables|Default|SetHoverEnabled (not (Variables|Default|GetHoverEnabled))))))
    (:false
      (Variables|Default|SetHoverEnabled false))))

(event EventSetHover
  (params (Value :type Boolean))
  (Variables|Default|SetHoverEnabled Value))