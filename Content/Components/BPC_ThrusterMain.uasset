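; BPC_ThrusterMain is a component that manages a ship's main thrust power across its thruster units.
; On BeginPlay it collects owner child actors implementing BPI_ThrusterUnit, then gathers their thrust data for the current power.
; Input ramps power between zero and one by the configured acceleration rate, only while thrust is enabled and unlocked.
; A separate function eases power toward zero using the configured dampening.
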(event EventBeginPlay
  (for _array_element (Actor|GetComponentsByClass (Components|GetOwner) "/Script/Engine.ChildActorComponent")
    (if (Utilities|DoesObjectImplementInterface (Variables|/Script/Engine.ChildActorComponent|GetChildActor _array_element) "/Game/Components/BPI_ThrusterUnit.BPI_ThrusterUnit_C")
      (Utilities|Array|Add (Variables|Default|GetThrusterUnits) (Variables|/Script/Engine.ChildActorComponent|GetChildActor _array_element)))))

(event EventLockThrusters
  (params (Value :type Boolean))
  (Variables|Flags|SetIsThrustLocked Value))

(event EventPowerThrusters
  (params (Value :type Boolean))
  (Variables|Flags|SetIsThrustEnabled Value))

(fn GetTotalThrust
  (for _array_element (Variables|Default|GetThrusterUnits)
    (bind _thrusterdata (Class|BPIThrusterUnit|GetThrusterData(Message) _array_element (Variables|Default|GetThrusterPower)))
    (Utilities|Array|Add (LocalVariables|GetThrusterData) _thrusterdata))
  (return (LocalVariables|GetThrusterData)))

(fn SetThrusterPower
  (params (ThrusterInput :type Float%20%28double-precision%29))
  (Utilities|ThrustOnline
    (:true
      (bind _output_get (Variables|Default|SetThrusterPower (Math|Float|Clamp(Float) (+ (Variables|Default|GetThrusterPower) (* ThrusterInput (.accelerationrate (Variables|Config|GetShipThrustConfig)) (Utilities|Time|GetWorldDeltaSeconds))))))
      (return _output_get))))

(fn SetThrusterZero
  (bind _output_get (Variables|Default|SetThrusterPower (Math|Interpolation|FInterpTo (Variables|Default|GetThrusterPower) 0.0 (Utilities|Time|GetWorldDeltaSeconds) (.dampening (Variables|Config|GetShipThrustConfig)))))
  (return _output_get))