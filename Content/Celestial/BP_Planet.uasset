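; BP_Planet is a planet actor that moves the player's ship from space onto a streamed surface level.
; An approach sphere preloads that level hidden and unloads it on exit unless the ship has landed in it.
; A transition sphere fades the camera out, teleports the ship to the surface spawn preserving velocity, and reveals the level.
; Arrival pitch steepens the more directly the ship faced the planet, then the camera fades back in.
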(event OnComponentBeginOverlap(ApproachSphere)
  (params (OverlappedComponent :type Primitive%20Component%20Object%20Reference) (OtherActor :type Actor%20Object%20Reference) (OtherComp :type Primitive%20Component%20Object%20Reference) (OtherBodyIndex :type Integer) (bFromSweep :type Boolean) (SweepResult :type Hit%20Result%20Structure%20%28by%20ref%29))
  (if (not (Variables|Default|GetSurfaceLoaded))
    (Game|LoadStreamLevel(byName) (Variables|Default|GetSurfaceLevelName) false)
    (Variables|Default|SetSurfaceLoaded true)))

(event OnComponentEndOverlap(ApproachSphere)
  (params (OverlappedComponent :type Primitive%20Component%20Object%20Reference) (OtherActor :type Actor%20Object%20Reference) (OtherComp :type Primitive%20Component%20Object%20Reference) (OtherBodyIndex :type Integer))
  (if (and (Variables|Default|GetSurfaceLoaded) (not (Variables|Default|GetShipInSurface)))
    (Game|UnloadStreamLevel(byName) (Variables|Default|GetSurfaceLevelName) false)
    (Variables|Default|SetSurfaceLoaded false)))

(event OnComponentBeginOverlap(TransitionSphere)
  (params (OverlappedComponent :type Primitive%20Component%20Object%20Reference) (OtherActor :type Actor%20Object%20Reference) (OtherComp :type Primitive%20Component%20Object%20Reference) (OtherBodyIndex :type Integer) (bFromSweep :type Boolean) (SweepResult :type Hit%20Result%20Structure%20%28by%20ref%29))
  (CallFunction|BeginCameraTransition))

(event Custom|BeginCameraTransition
  (bind _returnvalue (Game|GetPlayerCameraManager 0))
  (bind _returnvalue_2 (Game|Player|GetPlayerPawn 0))
  (Variables|Default|SetShipInSurface true)
  (CameraFades|StartCameraFade :self _returnvalue :ToAlpha 1.0 :Duration 0.3 :bShouldFadeAudio true :bHoldWhenFinished true)
  (Utilities|FlowControl|Delay 0.4)
  (bind _value (Class|BPIShipData|GetShipStatus(Message) _returnvalue_2))
  (bind _returnvalue_3 (Physics|GetPhysicsLinearVelocity (Utilities|Struct|BreakS_ShipData _value) "None"))
  (Transformation|SetActorLocation _returnvalue_2 (Variables|Default|GetSurfaceSpawnLocation) false true)
  (Physics|SetPhysicsLinearVelocity (Utilities|Struct|BreakS_ShipData _value) _returnvalue_3 false "None")
  (Variables|/Script/Engine.LevelStreaming|SetbShouldBeVisible (Class|GameplayStatics|GetStreamingLevel (Variables|Default|GetSurfaceLevelName)) true)
  (Transformation|SetActorRotation _returnvalue_2 (Math|Rotator|MakeRotator (.roll (Transformation|GetWorldRotation (Utilities|Struct|BreakS_ShipData _value))) (Math|Float|Lerp -3e+01 -9e+01 (Math|Float|Clamp(Float) (Math|Vector|DotProduct (Math|Vector|GetForwardVector (Utilities|Struct|BreakS_ShipData _value)) (Math|Vector|Normalize (- (Transformation|GetActorLocation) (Transformation|GetActorLocation _returnvalue_2)))))) (.yaw (Transformation|GetWorldRotation (Utilities|Struct|BreakS_ShipData _value)))))
  (Utilities|FlowControl|Delay 0.4)
  (CameraFades|StartCameraFade :self _returnvalue :FromAlpha 1.0 :ToAlpha 0.0 :Duration 0.3 :bShouldFadeAudio true :bHoldWhenFinished true))

(fn ConstructionScript)