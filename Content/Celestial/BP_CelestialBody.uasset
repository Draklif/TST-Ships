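; Data-driven planet or moon actor that orbits its parent, spins, and handles the ship's seamless space-to-surface travel.
; Approach sphere pre-streams the surface level hidden; transition sphere teleports the ship behind a fade, sets gravity and reveals it (both zero-radius for moons).
; On the surface, skybox proxies of other bodies and the directional light follow real orbital directions, rotated by axial spin and tilt.
; Orbit and sky updates are externally triggered.
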(event OnComponentBeginOverlap(ApproachSphere)
  (params (OverlappedComponent :type Primitive%20Component%20Object%20Reference) (OtherActor :type Actor%20Object%20Reference) (OtherComp :type Primitive%20Component%20Object%20Reference) (OtherBodyIndex :type Integer) (bFromSweep :type Boolean) (SweepResult :type Hit%20Result%20Structure%20%28by%20ref%29))
  ;[0.15 0.15 0.15 0.5] Overlap Events
  (Utilities|CanLoadSurface
    (:true
      (Game|LoadStreamLevel(byName) (.SurfaceLevelName (Utilities|Struct|BreakS_CelestialSurfaceData (.SurfaceData (Utilities|Struct|BreakS_CelestialBodyData (Variables|Default|GetCelestialBodyData))))) false)
      (Variables|Flags|SetSurfaceLoaded true))))

(event OnComponentEndOverlap(ApproachSphere)
  (params (OverlappedComponent :type Primitive%20Component%20Object%20Reference) (OtherActor :type Actor%20Object%20Reference) (OtherComp :type Primitive%20Component%20Object%20Reference) (OtherBodyIndex :type Integer))
  ;[0.15 0.15 0.15 0.5] Overlap Events
  (Utilities|CanUnloadSurface
    (:true
      (Game|UnloadStreamLevel(byName) (.SurfaceLevelName (Utilities|Struct|BreakS_CelestialSurfaceData (.SurfaceData (Utilities|Struct|BreakS_CelestialBodyData (Variables|Default|GetCelestialBodyData))))) false)
      (Variables|Flags|SetSurfaceLoaded false))))

(event OnComponentBeginOverlap(TransitionSphere)
  (params (OverlappedComponent :type Primitive%20Component%20Object%20Reference) (OtherActor :type Actor%20Object%20Reference) (OtherComp :type Primitive%20Component%20Object%20Reference) (OtherBodyIndex :type Integer) (bFromSweep :type Boolean) (SweepResult :type Hit%20Result%20Structure%20%28by%20ref%29))
  ;[0.15 0.15 0.15 0.5] Overlap Events
  (CallFunction|TransitiontoPlanet))

(event Custom|TransitionFromPlanet
  (Variables|Flags|SetShipInSurface false)
  (bind _output_get (Variables|References|SetPlayerRef (Game|Player|GetPlayerPawn 0)))
  (bind _value (Class|BPIShipData|GetShipData(Message) _output_get))
  (Variables|References|SetShipBodyRef (Utilities|Struct|BreakS_ShipData _value))
  (Utilities|FadeScreen 0.0 1.0 0.3)
  (Utilities|FlowControl|Delay 0.4)
  (CallFunction|ShipSetSurfaceData "NewEnumerator1" 0.0)
  (CallFunction|SetLevelVisibility (.SurfaceLevelName (Utilities|Struct|BreakS_CelestialSurfaceData (Utilities|Struct|BreakS_CelestialBodyData (Variables|Default|GetCelestialBodyData)))) false)
  (Class|BPISolarSystem|ToggleSystem(Message) (Variables|References|GetSolarSystemRef) true)
  (CallFunction|UnloadSkyboxMeshes)
  (Utilities|FlowControl|Delay 1.0)
  (Utilities|FadeScreen 1.0 0.0 0.3))

(event Custom|TransitionToPlanet
  (bind _celestialbodydata (Variables|Default|GetCelestialBodyData))
  (bind _surfacedata (Utilities|Struct|BreakS_CelestialBodyData _celestialbodydata))
  (bind (_surfacespawnlocation _surfaceentryinclination _surfacegravity _surfacelevelname) (Utilities|Struct|BreakS_CelestialSurfaceData _surfacedata))
  (Variables|Flags|SetShipInSurface true)
  (bind _output_get (Variables|References|SetPlayerRef (Game|Player|GetPlayerPawn 0)))
  (bind _value (Class|BPIShipData|GetShipData(Message) _output_get))
  (Variables|References|SetShipBodyRef (Utilities|Struct|BreakS_ShipData _value))
  (Utilities|CheckShipFlag "NewEnumerator2"
    (:true
      _)
    (:false
      (Utilities|FadeScreen 0.0 1.0 0.3)))
  (Utilities|FlowControl|Delay 0.4)
  (CallFunction|ShipToggleComponents false)
  (CallFunction|ShipTeleportandRotation _surfacespawnlocation _surfaceentryinclination)
  (CallFunction|ShipSetSurfaceData "NewEnumerator2" _surfacegravity)
  (CallFunction|SetLevelVisibility _surfacelevelname true)
  (Class|BPISolarSystem|ToggleSystem(Message) (Variables|References|GetSolarSystemRef) false)
  (CallFunction|LoadSkyboxMeshes)
  (Utilities|FlowControl|Delay 1.0)
  (Utilities|CheckShipFlag "NewEnumerator2"
    (:false
      (Utilities|FadeScreen 1.0 0.0 0.3))))

(event EventUpdateSkyBox
  (CallFunction|UpdateSkyboxMeshes)
  (CallFunction|UpdateSkyboxSun))

(event EventUpdateOrbit
  (params (DeltaTime :type Float%20%28double-precision%29))
  (CallFunction|UpdateOrbitPlanet DeltaTime))

(event EventBeginPlay
  (bind _celestialbodydata (Variables|Default|GetCelestialBodyData))
  (bind (_type _initialangle) (Utilities|Struct|BreakS_CelestialBodyData _celestialbodydata))
  (Variables|Default|SetCurrentAngle _initialangle)
  (bind _returnvalue (Actor|GetActorOfClass "/Game/Celestial/BP_SolarSystemManager.BP_SolarSystemManager_C"))
  (Variables|References|SetSolarSystemRef _returnvalue)
  (Variables|References|SetSunPosition (Transformation|GetActorLocation _returnvalue))
  (switch Utilities|FlowControl|Switch|SwitchonE_BodyType _type
    (:NewEnumerator6
      (Components|Sphere|SetSphereRadius (Variables|Default|GetApproachSphere) 0.0 true)
      (Components|Sphere|SetSphereRadius (Variables|Default|GetTransitionSphere) 0.0 true))))

(fn ConstructionScript)

(fn LoadSkyboxMeshes
  (bind _returnvalue (Actor|GetActorOfClass "/Script/Engine.DirectionalLight"))
  (Variables|References|SetSunLightRef _returnvalue)
  (bind _bodies (Class|BPISolarSystem|GetCelestialBodies(Message) (Variables|References|GetSolarSystemRef)))
  (for _array_element _bodies
    (if (!= _array_element self)
      (bind _returnvalue_2 (Game|SpawnActorfromClass "/Game/Celestial/BP_SkyboxRepresentation.BP_SkyboxRepresentation_C" (Math|Transform|MakeTransform "0, 0, 0") "Undefined" "MultiplyWithRoot" 0 (.SkyboxRepresentation (Utilities|Struct|BreakS_CelestialBodyData (Variables|BP_CelestialBody_C|GetCelestialBodyData _array_element))) 0))
      (Transformation|SetActorScale3D _returnvalue_2 (Variables|/Script/Engine.SceneComponent|GetRelativeScale3D (Variables|BP_CelestialBody_C|GetPlanet _array_element)))
      (Utilities|Map|Add (Variables|Default|GetSpawnedSkyMeshes) _array_element _returnvalue_2))))

(fn UnloadSkyboxMeshes
  (bind _spawnedskymeshes (Variables|Default|GetSpawnedSkyMeshes))
  (bind _valuepin (Utilities|Map|ForEachLoop(Map) _spawnedskymeshes)
    (:then
      (Actor|DestroyActor _valuepin))
    (:CompletedPin
      (Utilities|Map|Clear _spawnedskymeshes))))

(fn UpdateSkyboxSun
  (Utilities|IsValid (Variables|References|GetSunLightRef)
    (:Is%20Valid
      _)
    (:Is%20Not%20Valid
      (bind _returnvalue (Actor|GetActorOfClass "/Script/Engine.DirectionalLight"))
      (bind _output_get (Variables|References|SetSunLightRef _returnvalue))
      (Utilities|IsValid _output_get
        (:Is%20Valid
          _))))
  (Transformation|SetActorRotation (Variables|References|GetSunLightRef) (Math|Rotator|MakeRotfromX (Math|Vector|RotateVector (Math|Vector|RotateVector (Math|Vector|Normalize (- (Variables|References|GetSunPosition) (Transformation|GetActorLocation))) (Math|Rotator|MakeRotator 0.0 0.0 (Variables|Default|GetCurrentAxialAngle))) (Math|Rotator|MakeRotator 0.0 (.AxialTilt (Utilities|Struct|BreakS_CelestialBodyData (Variables|Default|GetCelestialBodyData))) 0.0)))))

(fn UpdateSkyboxMeshes
  (bind _returnvalue (Game|Player|GetPlayerPawn 0))
  (bind _returnvalue_2 (Transformation|GetActorLocation _returnvalue))
  (bind (_keypin _valuepin) (Utilities|Map|ForEachLoop(Map) (Variables|Default|GetSpawnedSkyMeshes))
    (:then
      (Transformation|SetActorLocation _valuepin (+ (Math|Vector|MakeVector (.x _returnvalue_2) (.y _returnvalue_2) 0.0) (* (Math|Vector|RotateVector (Math|Vector|RotateVector (Math|Vector|Normalize (- (Transformation|GetActorLocation _keypin) (Transformation|GetActorLocation))) (Math|Rotator|MakeRotator 0.0 0.0 (Variables|Default|GetCurrentAxialAngle))) (Math|Rotator|MakeRotator 0.0 (.AxialTilt (Utilities|Struct|BreakS_CelestialBodyData (Variables|Default|GetCelestialBodyData))) 0.0)) (/ (Math|Vector|VectorLength (- (Transformation|GetActorLocation _keypin) (Transformation|GetActorLocation))) (Variables|Default|GetDistanceDivisor)))) false false))))

(fn UpdateOrbitPlanet
  (params (InputPin :type Float%20%28double-precision%29))
  (bind _celestialbodydata (Variables|Default|GetCelestialBodyData))
  (bind (_type _orbitparent _orbitradius _orbitspeed _orbitinclination _axialrotationspeed) (Utilities|Struct|BreakS_CelestialBodyData _celestialbodydata))
  (bind _returnvalue (* InputPin _axialrotationspeed))
  (Variables|Default|SetCurrentAngle (+ (Variables|Default|GetCurrentAngle) (* InputPin _orbitspeed)))
  (Transformation|SetActorLocation (+ (Math|Vector|MakeVector (* _orbitradius (Math|Trig|Cos(Degrees) (Variables|Default|GetCurrentAngle))) (* _orbitradius (Math|Trig|Sin(Degrees) (Variables|Default|GetCurrentAngle))) (* _orbitradius (Math|Trig|Sin(Degrees) (Variables|Default|GetCurrentAngle)) (Math|Trig|Sin(Radians) _orbitinclination))) (Transformation|GetActorLocation _orbitparent)) false false)
  (Variables|Default|SetCurrentAxialAngle (+ (Variables|Default|GetCurrentAxialAngle) _returnvalue))
  (Transformation|AddActorLocalRotation (Math|Rotator|MakeRotator 0.0 0.0 _returnvalue) false false))

(fn ShipTeleportandRotation
  (params (EntryLocation :type Vector) (EntryInclination :type Float%20%28single-precision%29))
  (bind _playerref (Variables|References|GetPlayerRef)
    (:then
      (bind _shipbodyref (Variables|References|GetShipBodyRef)
        (:then
          (bind _returnvalue (Physics|GetPhysicsLinearVelocity _shipbodyref "None"))
          (LocalVariables|SetVelocity _returnvalue)
          (Transformation|SetActorLocation _playerref EntryLocation false false)
          (Physics|SetPhysicsLinearVelocity _shipbodyref (LocalVariables|GetVelocity) false "None")
          (Transformation|SetActorRotation _playerref (Math|Rotator|MakeRotator 0.0 EntryInclination (.yaw (Transformation|GetActorRotation _playerref)))))
        (:else)))
    (:else)))

(fn ShipToggleComponents
  (params (Value :type Boolean))
  (bind _playerref (Variables|References|GetPlayerRef)
    (:then
      (Utilities|IsValid _playerref
        (:Is%20Valid
          (Class|BPIShipControls|SetRemoteComponent(Message) _playerref "/Game/Components/BPC_Stabilizer.BPC_Stabilizer_C" Value)
          (Class|BPIShipControls|SetRemoteComponent(Message) _playerref "/Game/Components/BPC_Lock.BPC_Lock_C" Value))))
    (:else)))

(fn ShipSetSurfaceData
  (params (LocationState :type E_ShipLocationState%20Enum :default "NewEnumerator0") (SurfaceGravity :type Float%20%28double-precision%29))
  (bind _playerref (Variables|References|GetPlayerRef)
    (:then
      (Class|BPIShipData|SetLocationState(Message) _playerref LocationState)
      (Class|BPIShipControls|SetGravity(Message) _playerref SurfaceGravity)
      (Class|BPIShipData|SetCurrentPlanet(Message) _playerref self))
    (:else)))

(fn SetLevelVisibility
  (params (PackageName :type Name) (Should%20be%20Visible :type Boolean))
  (Variables|/Script/Engine.LevelStreaming|SetbShouldBeVisible (Class|GameplayStatics|GetStreamingLevel PackageName) Should%20be%20Visible))

(fn GetDisplayName
  (return ""))

(fn GetLockonLocation
  (return (Transformation|GetActorLocation)))

(fn GetLockType
  (return (Utilities|Struct|BreakS_CelestialBodyData (Variables|Default|GetCelestialBodyData))))