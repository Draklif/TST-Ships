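; Solar system manager actor that drives the orbital simulation of every BP_CelestialBody in the level.
; It gathers the bodies on BeginPlay, then each tick advances their orbits by scaled delta time unless paused.
; Bodies flagged as having the ship on their surface also update their skybox during that tick.
; ToggleSystem shows or hides the planets and Sun with their children, and GetCelestialBodies exposes the cached list.
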(event EventBeginPlay
  (bind _outactors (Actor|GetAllActorsOfClass "/Game/Celestial/BP_CelestialBody.BP_CelestialBody_C"))
  (Variables|Default|SetBodies _outactors))

(event EventTick
  (params (DeltaSeconds :type Float%20%28single-precision%29))
  (if (not (Variables|Default|GetSystemPaused))
    (for _array_element (Variables|Default|GetBodies)
      (Class|BPICelestialBody|UpdateOrbit(Message) _array_element (* (Variables|Default|GetTimeScale) DeltaSeconds))
      (if (Variables|/Game/Celestial/BP_CelestialBody.BP_CelestialBody_C|GetShipInSurface _array_element)
        (Class|BPICelestialBody|UpdateSkyBox(Message) _array_element)))))

(event EventToggleSystem
  (params (Value :type Boolean))
  (for _array_element (Variables|Default|GetBodies)
    (Rendering|SetVisibility (Variables|/Game/Celestial/BP_CelestialBody.BP_CelestialBody_C|GetPlanet _array_element) Value true)
    (Rendering|SetVisibility (Variables|Default|GetSun) Value true)))

(fn ConstructionScript)

(fn GetCelestialBodies
  (return (Variables|Default|GetBodies)))