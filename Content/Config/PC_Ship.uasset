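; PC_Ship is a player controller that handles input for a flyable ship.
; On BeginPlay it adds the ship's Enhanced Input mapping context, then relays each action to the controlled pawn as a message call, keeping flight logic out of the controller.
; Look and roll forward their values, while move and climb send a value on start and zero on completion.
; Mode actions such as hover, land and warp send only true on press.
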(event Input|EnhancedActionEvents|EnhancedInputActionIA_LookX
  (params (ActionValue :type Float%20%28double-precision%29) (ElapsedSeconds :type Float%20%28double-precision%29) (TriggeredSeconds :type Float%20%28double-precision%29) (InputAction :type Input%20Action%20Object%20Reference :default "/Game/Inputs/IA_LookX.IA_LookX"))
  (Class|BPIShipControls|LookX(Message) (Pawn|GetControlledPawn) ActionValue))

(event Input|EnhancedActionEvents|EnhancedInputActionIA_LookY
  (params (ActionValue :type Float%20%28double-precision%29) (ElapsedSeconds :type Float%20%28double-precision%29) (TriggeredSeconds :type Float%20%28double-precision%29) (InputAction :type Input%20Action%20Object%20Reference :default "/Game/Inputs/IA_LookY.IA_LookY"))
  (Class|BPIShipControls|LookY(Message) (Pawn|GetControlledPawn) ActionValue))

(event Input|EnhancedActionEvents|EnhancedInputActionIA_Lock
  (params (ActionValue :type Boolean) (ElapsedSeconds :type Float%20%28double-precision%29) (TriggeredSeconds :type Float%20%28double-precision%29) (InputAction :type Input%20Action%20Object%20Reference :default "/Game/Inputs/IA_Lock.IA_Lock"))
  (:Started
    (Class|BPIShipControls|Lock(Message) (Pawn|GetControlledPawn) true)))

(event Input|EnhancedActionEvents|EnhancedInputActionIA_Warp
  (params (ActionValue :type Boolean) (ElapsedSeconds :type Float%20%28double-precision%29) (TriggeredSeconds :type Float%20%28double-precision%29) (InputAction :type Input%20Action%20Object%20Reference :default "/Game/Inputs/IA_Warp.IA_Warp"))
  (:Started
    (Class|BPIShipControls|Warp(Message) (Pawn|GetControlledPawn) true)))

(event Input|EnhancedActionEvents|EnhancedInputActionIA_Roll
  (params (ActionValue :type Float%20%28double-precision%29) (ElapsedSeconds :type Float%20%28double-precision%29) (TriggeredSeconds :type Float%20%28double-precision%29) (InputAction :type Input%20Action%20Object%20Reference :default "/Game/Inputs/IA_Roll.IA_Roll"))
  (Class|BPIShipControls|Roll(Message) (Pawn|GetControlledPawn) ActionValue))

(event Input|EnhancedActionEvents|EnhancedInputActionIA_Move
  (params (ActionValue :type Float%20%28double-precision%29) (ElapsedSeconds :type Float%20%28double-precision%29) (TriggeredSeconds :type Float%20%28double-precision%29) (InputAction :type Input%20Action%20Object%20Reference :default "/Game/Inputs/IA_Move.IA_Move"))
  (bind _returnvalue (Pawn|GetControlledPawn))
  (:Started
    (Class|BPIShipControls|Move(Message) _returnvalue ActionValue))
  (:Completed
    (Class|BPIShipControls|Move(Message) _returnvalue 0.0)))

(event Input|EnhancedActionEvents|EnhancedInputActionIA_Stabilize
  (params (ActionValue :type Boolean) (ElapsedSeconds :type Float%20%28double-precision%29) (TriggeredSeconds :type Float%20%28double-precision%29) (InputAction :type Input%20Action%20Object%20Reference :default "/Game/Inputs/IA_Stabilize.IA_Stabilize"))
  (:Started
    (Class|BPIShipControls|Stabilize(Message) (Pawn|GetControlledPawn) true)))

(event Input|EnhancedActionEvents|EnhancedInputActionIA_Climb
  (params (ActionValue :type Float%20%28double-precision%29) (ElapsedSeconds :type Float%20%28double-precision%29) (TriggeredSeconds :type Float%20%28double-precision%29) (InputAction :type Input%20Action%20Object%20Reference :default "/Game/Inputs/IA_Climb.IA_Climb"))
  (bind _returnvalue (Pawn|GetControlledPawn))
  (:Started
    (Class|BPIShipControls|Climb(Message) _returnvalue ActionValue))
  (:Completed
    (Class|BPIShipControls|Climb(Message) _returnvalue 0.0)))

(event Input|EnhancedActionEvents|EnhancedInputActionIA_Power
  (params (ActionValue :type Boolean) (ElapsedSeconds :type Float%20%28double-precision%29) (TriggeredSeconds :type Float%20%28double-precision%29) (InputAction :type Input%20Action%20Object%20Reference :default "/Game/Inputs/IA_Power.IA_Power"))
  (:Started
    (Class|BPIShipControls|Power(Message) (Pawn|GetControlledPawn) true)))

(event Input|EnhancedActionEvents|EnhancedInputActionIA_Hover
  (params (ActionValue :type Boolean) (ElapsedSeconds :type Float%20%28double-precision%29) (TriggeredSeconds :type Float%20%28double-precision%29) (InputAction :type Input%20Action%20Object%20Reference :default "/Game/Inputs/IA_Hover.IA_Hover"))
  (:Started
    (Class|BPIShipControls|Hover(Message) (Pawn|GetControlledPawn) true)))

(event Input|EnhancedActionEvents|EnhancedInputActionIA_Land
  (params (ActionValue :type Boolean) (ElapsedSeconds :type Float%20%28double-precision%29) (TriggeredSeconds :type Float%20%28double-precision%29) (InputAction :type Input%20Action%20Object%20Reference :default "/Game/Inputs/IA_Land.IA_Land"))
  (:Started
    (Class|BPIShipControls|Land(Message) (Pawn|GetControlledPawn) true)))

(event Input|EnhancedActionEvents|EnhancedInputActionIA_FreeCam
  (params (ActionValue :type Boolean) (ElapsedSeconds :type Float%20%28double-precision%29) (TriggeredSeconds :type Float%20%28double-precision%29) (InputAction :type Input%20Action%20Object%20Reference :default "/Game/Inputs/IA_FreeCam.IA_FreeCam"))
  (:Started
    (Class|BPIShipControls|FreeCam(Message) (Pawn|GetControlledPawn) true)))

(event EventBeginPlay
  (Input|AddMappingContext (PlayerController|LocalPlayerSubsystems|GetEnhancedInputLocalPlayerSubsystem) "/Game/Inputs/IMC_Ship.IMC_Ship" 0 "(bIgnoreAllPressedKeysUntilRelease=True,bForceImmediately=False,bNotifyUserSettings=False)"))

(fn ConstructionScript)