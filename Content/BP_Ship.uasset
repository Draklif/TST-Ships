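; Player-controlled physics ship that flies on thruster impulses and gravity, with power, landing, launch and free-camera controls.
; Input is routed to optional components (camera, torque, thrusters, stabilizer, hover, landing, FCS), looked up by class and driven through message calls.
; While not landed, Tick applies gravity with a ground trace, stabilization, damping, then per-thruster impulses, balanced by the FCS if present.
; A debug key simulates a side impact.
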(event OnComponentHit(Ship)
  (params (HitComponent :type Primitive%20Component%20Object%20Reference) (OtherActor :type Actor%20Object%20Reference) (OtherComp :type Primitive%20Component%20Object%20Reference) (NormalImpulse :type Vector :default "0, 0, 0") (Hit :type Hit%20Result%20Structure%20%28by%20ref%29)))

(event EventPowerOff
  (Variables|Flags|SetIsShipOnline false)
  (CallFunction|TurnSystems false))

(event EventPoweron
  (Variables|Flags|SetIsShipOnline true)
  (CallFunction|TurnSystems true))

(event EventPower
  (params (Value :type Boolean))
  (bind _output_get (Variables|Flags|SetIsShipOnline (not (Variables|Flags|GetIsShipOnline))))
  (if _output_get
    (CallFunction|Poweron)
    (else
      (CallFunction|PowerOff))))

(event EventHover
  (params (Value :type Boolean))
  (bind _output (Utilities|HasComponent "/Game/Components/BPC_Hover.BPC_Hover_C")
    (:Is%20Valid
      (Class|BPIHover|ToggleHover(Message) _output))))

(event EventLand
  (params (Value :type Boolean))
  (bind _output (Utilities|HasComponent "/Game/Components/BPC_Landing.BPC_Landing_C")
    (:Is%20Valid
      (Class|BPILanding|InitSequence(Message) _output))))

(event EventFreeCam
  (params (Value :type Boolean))
  (bind _output (Utilities|HasComponent "/Game/Components/BPC_Camera.BPC_Camera_C")
    (:Is%20Valid
      (Class|BPICamera|ToggleFreeCam(Message) _output))))

(event EventSetIsLanded
  (params (Value :type Boolean))
  (Variables|Flags|SetIsShipLanded Value))

(event EventLookY
  (params (Value :type Float%20%28double-precision%29))
  (bind _output (Utilities|HasComponent "/Game/Components/BPC_Camera.BPC_Camera_C")
    (:Is%20Valid
      (bind _value (Class|BPICamera|GetIsFreeCam(Message) _output))
      (if _value
        (Class|BPICamera|SetCameraPitch(Message) _output Value)
        (else
          (bind _output_2 (Utilities|HasComponent "/Game/Components/BPC_Torque.BPC_Torque_C" :!label _label)
            (:Is%20Valid
              (Class|BPITorque|HandleRotation(Message) _output_2 Value "NewEnumerator0"))))))
    (:Is%20Not%20Valid
      (goto _label))))

(event EventLookX
  (params (Value :type Float%20%28double-precision%29))
  (bind _output (Utilities|HasComponent "/Game/Components/BPC_Camera.BPC_Camera_C")
    (:Is%20Valid
      (bind _value (Class|BPICamera|GetIsFreeCam(Message) _output))
      (if _value
        (Class|BPICamera|SetCameraYaw(Message) _output Value)
        (else
          (bind _output_2 (Utilities|HasComponent "/Game/Components/BPC_Torque.BPC_Torque_C" :!label _label)
            (:Is%20Valid
              (Class|BPITorque|HandleRotation(Message) _output_2 Value "NewEnumerator2"))))))
    (:Is%20Not%20Valid
      (goto _label))))

(event EventRoll
  (params (Value :type Float%20%28double-precision%29))
  (bind _output (Utilities|HasComponent "/Game/Components/BPC_Torque.BPC_Torque_C")
    (:Is%20Valid
      (Class|BPITorque|HandleRotation(Message) _output Value "NewEnumerator1"))))

(event EventMove
  (params (Value :type Float%20%28double-precision%29))
  (Utilities|ShipOnline
    (:true
      (Utilities|ShipLanded
        (:true
          (bind _output (Utilities|HasComponent "/Game/Components/BPC_Landing.BPC_Landing_C")
            (:Is%20Valid
              (Class|BPILanding|LaunchSequence(Message) _output))))
        (:false
          (Variables|Thrust|SetDriveInput Value))))
    (:false
      (Variables|Thrust|SetDriveInput -1.0))))

(event EventTick
  (params (DeltaSeconds :type Float%20%28single-precision%29))
  (Utilities|ShipLanded
    (:false
      (CallFunction|ApplyGravity)
      (Utilities|FlowControl|Sequence
        (:then_0
          (bind _output (Utilities|HasComponent "/Game/Components/BPC_Stabilizer.BPC_Stabilizer_C")
            (:Is%20Valid
              (Class|BPIStabilizer|StabilizeTick(Message) _output))))
        (:then_1
          (CallFunction|ApplyLinearDamping))
        (:then_2
          (CallFunction|HandleThrusters))))))

(event EventStabilize
  (params (Value :type Boolean))
  (bind _output (Utilities|HasComponent "/Game/Components/BPC_Stabilizer.BPC_Stabilizer_C")
    (:Is%20Valid
      (Class|BPIStabilizer|ToggleStabilizer(Message) _output))))

(event EventClimb
  (params (Value :type Float%20%28double-precision%29))
  (Utilities|ShipOnline
    (:true
      (Utilities|ShipLanded
        (:true
          (bind _output (Utilities|HasComponent "/Game/Components/BPC_Landing.BPC_Landing_C")
            (:Is%20Valid
              (Class|BPILanding|LaunchSequence(Message) _output))))
        (:false
          (Variables|Thrust|SetLiftInput Value))))
    (:false
      (Variables|Thrust|SetLiftInput 0.0))))

(event Input|KeyboardEvents|DebugKeyTab
  (params (Key :type Key%20Structure :default "None") (ActionValue :type Input%20Action%20Value%20Structure))
  (bind _returnvalue (Transformation|GetActorLocation))
  (bind _ship (Variables|Default|GetShip))
  (bind _returnvalue_2 (Math|Vector|GetRightVector _ship))
  (bind _returnvalue_3 (* _returnvalue_2 5e+02))
  (bind _returnvalue_4 (* _returnvalue_2 -1.0 5e+03))
  (bind _returnvalue_5 (+ _returnvalue _returnvalue_3))
  (:Pressed
    (Collision|LineTraceByChannel _returnvalue_5 (+ _returnvalue_5 _returnvalue_4) "TraceTypeQuery1" false 0 "ForDuration" false)
    (Physics|AddImpulse (Variables|Default|GetShip) _returnvalue_4 "None" true)
    (Camera|PlayWorldCameraShake "/Game/BP_Shake.BP_Shake_C" (Transformation|GetActorLocation) 0.0 2e+04)
    (Class|PrimitiveComponent|AddTorqueinDegrees (Variables|Default|GetShip) (* (Math|Random|RandomUnitVector) 5e+03) "None" true)))

(fn ConstructionScript)

(fn ApplyGravity
  (bind _returnvalue (Transformation|GetActorLocation))
  (Utilities|ShipinSpace
    (:false
      (bind _returnvalue_2 (Collision|LineTraceByChannel _returnvalue (+ _returnvalue "0.000000,0.000000,-150.000000") "TraceTypeQuery1" false 0 "ForOneFrame"))
      (if _returnvalue_2
        (Utilities|ShipOnline
          (:true
            (bind _output (Utilities|HasComponent "/Game/Components/BPC_Stabilizer.BPC_Stabilizer_C")
              (:Is%20Valid
                (Class|BPIStabilizer|SetStabilizer(Message) _output false))))
          (:false
            (bind _output_2 (Utilities|HasComponent "/Game/Components/BPC_Landing.BPC_Landing_C")
              (:Is%20Valid
                (Class|BPILanding|LandSequence(Message) _output_2)))))
        (else
          (Physics|AddImpulse (Variables|Default|GetShip) (Math|Vector|MakeVector 0.0 0.0 (* (Variables|Default|GetCurrentGravity) -1.0 (Utilities|Time|GetWorldDeltaSeconds))) "None" true))))))

(fn ApplyLinearDamping
  (bind _ship (Variables|Default|GetShip))
  (Utilities|ShipOnline
    (:true
      (Class|PrimitiveComponent|SetLinearDamping _ship 0.5))
    (:false
      (Class|PrimitiveComponent|SetLinearDamping _ship 0.5))))

(fn HandleThrusters
  (bind _liftinput (Variables|Thrust|GetLiftInput))
  (bind _ship (Variables|Default|GetShip))
  (bind _ship_2 (Variables|Default|GetShip))
  (bind _output (Utilities|HasComponent "/Game/Components/BPC_Thrusters.BPC_Thrusters_C")
    (:Is%20Valid
      (Utilities|ShipOnline
        (:true
          (Class|BPIThrusters|SetDrivePower(Message) _output (Variables|Thrust|GetDriveInput)))
        (:false
          (Class|BPIThrusters|SetDriveZero(Message) _output)))
      (if (!= _liftinput 0.0)
        (Class|BPIThrusters|SetLiftPower(Message) _output _liftinput)
        (else
          (Class|BPIThrusters|SetLiftZero(Message) _output)))
      (bind _thrusterdata (Class|BPIThrusters|GetThrusterData(Message) _output))
      (LocalVariables|SetThrusterData _thrusterdata)
      ;[0.15 0.15 0.15 0.5] Try FCS if available
      (bind _output_2 (Utilities|HasComponent "/Game/Components/BPC_FCS.BPC_FCS_C")
        (:Is%20Valid
          (bind _balanceddata (Class|BPIFCS|BalanceThrusters(Message) _output_2 (LocalVariables|GetThrusterData)))
          (LocalVariables|SetThrusterData _balanceddata))
        (:Is%20Not%20Valid
          _))
      ;[0.15 0.15 0.15 0.5] Apply Impulse at every thruster
      (for _array_element (LocalVariables|GetThrusterData)
        (switch Utilities|FlowControl|Switch|SwitchonE_ThrusterType (.type _array_element)
          (:NewEnumerator0
            (Physics|AddImpulseatLocation _ship_2 (* (.thrust _array_element) (Math|Vector|GetForwardVector _ship_2)) (.location _array_element) "None"))
          (:NewEnumerator1
            (Physics|AddImpulse _ship (* (.thrust _array_element) (Math|Vector|GetUpVector _ship)) "None" true)))))))

(fn TurnSystems
  (params (Value :type Boolean))
  (Utilities|FlowControl|Sequence
    (:then_0
      (bind _output (Utilities|HasComponent "/Game/Components/BPC_FCS.BPC_FCS_C")
        (:Is%20Valid
          (Class|BPIFCS|SetFCS(Message) _output Value))))
    (:then_1
      (bind _output_2 (Utilities|HasComponent "/Game/Components/BPC_Stabilizer.BPC_Stabilizer_C")
        (:Is%20Valid
          (Class|BPIStabilizer|SetStabilizer(Message) _output_2 Value))))
    (:then_2
      (bind _output_3 (Utilities|HasComponent "/Game/Components/BPC_Hover.BPC_Hover_C")
        (:Is%20Valid
          (Class|BPIHover|SetHover(Message) _output_3 Value))))))

(fn GetShipStatus
  (return (Utilities|Struct|MakeS_ShipData (Variables|Flags|GetIsShipOnline) (Variables|Flags|GetIsShipLanded) (Variables|Flags|GetIsShipInSpace) (Variables|Default|GetShip) (Variables|Default|GetCurrentGravity))))

(fn GetSpringArm
  (return (Variables|Default|GetSpringArm)))